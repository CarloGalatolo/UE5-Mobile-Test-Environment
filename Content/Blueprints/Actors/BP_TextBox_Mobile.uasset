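; Mobile text box actor that shows per-instance text lines in a popup UI widget.
; The game instance's controls type picks the trigger: sphere overlap for Joysticks, touching the info point for 360° Media.
; Both paths stop player movement, create WBP_TextBox_UI stored on the first-person character, and fill it from TextLines.
; It then plays a pop sound, switches to UI-only input and hides the joystick and controls UI.
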(event OnInputTouchEnd(InfoPoint)
  (params (FingerIndex :type ETouchIndex%20Enum :default "Touch1") (TouchedComponent :type Primitive%20Component%20Object%20Reference))
  (bind _returnvalue (Game|GetPlayerController 0))
  (bind _returnvalue_2 (Game|GetPlayerCharacter 0))
  (bind _returnvalue_3 (Game|GetPlayerController 0))
  (bind _asbp_first_person_character (Utilities|Casting|CastToBP_FirstPersonCharacter _returnvalue_2))
  (switch Utilities|FlowControl|Switch|SwitchonEnum_ControlTypes (CallFunction|GetGlobalControlsType)
    (:NewEnumerator0
      ;[1 1 1] Show Text Widget
      (AI|Navigation|StopMovement _returnvalue_3)
      (bind _returnvalue_4 (UserInterface|CreateWidget "/Game/Blueprints/UI/WBP_TextBox_UI.WBP_TextBox_UI_C" _returnvalue_3))
      (bind _output_get (Variables|/Game/Blueprints/Game/BP_FirstPersonCharacter.BP_FirstPersonCharacter_C|SetWBP%20Text%20Box%20UI%20Reference _asbp_first_person_character _returnvalue_4))
      ;[0.7758 0.1981 0.3916] Builds text appending strings. Separates string with empty lines.
      ; (Carriage return chars don't work inside editor's text boxes)
      (Variables|/Script/UMG.MultiLineEditableText|SetText (Variables|/Game/Blueprints/UI/WBP_TextBox_UI.WBP_TextBox_UI_C|GetEditableText _output_get) "")
      (for (_array_element _array_index) (Variables|Default|GetText%20Lines)
        (if (== _array_index 0)
          (Variables|/Script/UMG.MultiLineEditableText|SetText (Variables|/Game/Blueprints/UI/WBP_TextBox_UI.WBP_TextBox_UI_C|GetEditableText _output_get) (Utilities|Text|ToText(String) (Utilities|String|Append (Utilities|String|ToString(Text) (Class|MultiLineEditableText|GetText (Variables|/Game/Blueprints/UI/WBP_TextBox_UI.WBP_TextBox_UI_C|GetEditableText _output_get))) (Utilities|String|ToString(Text) _array_element))))
          (else
            (Variables|/Script/UMG.MultiLineEditableText|SetText (Variables|/Game/Blueprints/UI/WBP_TextBox_UI.WBP_TextBox_UI_C|GetEditableText _output_get) (Utilities|Text|ToText(String) (Utilities|String|Append (Utilities|String|ToString(Text) (Class|MultiLineEditableText|GetText (Variables|/Game/Blueprints/UI/WBP_TextBox_UI.WBP_TextBox_UI_C|GetEditableText _output_get))) " 
" (Utilities|String|ToString(Text) _array_element)))))))
      ;[1 1 1] Hide input UI
      (Audio|PlaySound2D "/Game/Audio/SFX/Blueprints_TextPop03.Blueprints_TextPop03" 1.0 1.0 0.0 0 0)
      (UserInterface|Viewport|AddtoViewport _output_get 0)
      (Input|SetInputModeUIOnly _returnvalue 0 "DoNotLock" true)
      (Class|PlayerController|SetVirtualJoystickVisibility _returnvalue false)
      (Widget|RemovefromParent (Variables|/Game/Blueprints/Game/BP_FirstPersonCharacter.BP_FirstPersonCharacter_C|GetUI%20Controls%20Reference _asbp_first_person_character)))))

(event OnComponentBeginOverlap(Trigger)
  (params (OverlappedComponent :type Primitive%20Component%20Object%20Reference) (OtherActor :type Actor%20Object%20Reference) (OtherComp :type Primitive%20Component%20Object%20Reference) (OtherBodyIndex :type Integer) (bFromSweep :type Boolean) (SweepResult :type Hit%20Result%20Structure%20%28by%20ref%29))
  (bind _returnvalue (Game|GetPlayerController 0))
  (bind _returnvalue_2 (Game|GetPlayerCharacter 0))
  (bind _returnvalue_3 (Game|GetPlayerController 0))
  (bind _asbp_first_person_character (Utilities|Casting|CastToBP_FirstPersonCharacter _returnvalue_2))
  (switch Utilities|FlowControl|Switch|SwitchonEnum_ControlTypes (CallFunction|GetGlobalControlsType)
    (:NewEnumerator1
      ;[1 1 1] Show Text Widget
      (AI|Navigation|StopMovement _returnvalue_3)
      (bind _returnvalue_4 (UserInterface|CreateWidget "/Game/Blueprints/UI/WBP_TextBox_UI.WBP_TextBox_UI_C" _returnvalue_3))
      (bind _output_get (Variables|/Game/Blueprints/Game/BP_FirstPersonCharacter.BP_FirstPersonCharacter_C|SetWBP%20Text%20Box%20UI%20Reference _asbp_first_person_character _returnvalue_4))
      ;[0.7758 0.1981 0.3916] Builds text appending strings. Separates string with empty lines.
      ; (Carriage return chars don't work inside editor's text boxes)
      (Variables|/Script/UMG.MultiLineEditableText|SetText (Variables|/Game/Blueprints/UI/WBP_TextBox_UI.WBP_TextBox_UI_C|GetEditableText _output_get) "")
      (for (_array_element _array_index) (Variables|Default|GetText%20Lines)
        (if (== _array_index 0)
          (Variables|/Script/UMG.MultiLineEditableText|SetText (Variables|/Game/Blueprints/UI/WBP_TextBox_UI.WBP_TextBox_UI_C|GetEditableText _output_get) (Utilities|Text|ToText(String) (Utilities|String|Append (Utilities|String|ToString(Text) (Class|MultiLineEditableText|GetText (Variables|/Game/Blueprints/UI/WBP_TextBox_UI.WBP_TextBox_UI_C|GetEditableText _output_get))) (Utilities|String|ToString(Text) _array_element))))
          (else
            (Variables|/Script/UMG.MultiLineEditableText|SetText (Variables|/Game/Blueprints/UI/WBP_TextBox_UI.WBP_TextBox_UI_C|GetEditableText _output_get) (Utilities|Text|ToText(String) (Utilities|String|Append (Utilities|String|ToString(Text) (Class|MultiLineEditableText|GetText (Variables|/Game/Blueprints/UI/WBP_TextBox_UI.WBP_TextBox_UI_C|GetEditableText _output_get))) " 
" (Utilities|String|ToString(Text) _array_element)))))))
      ;[1 1 1] Hide input UI
      (Audio|PlaySound2D "/Game/Audio/SFX/Blueprints_TextPop03.Blueprints_TextPop03" 1.0 1.0 0.0 0 0)
      (UserInterface|Viewport|AddtoViewport _output_get 0)
      (Input|SetInputModeUIOnly _returnvalue 0 "DoNotLock" true)
      (Class|PlayerController|SetVirtualJoystickVisibility _returnvalue false)
      (Widget|RemovefromParent (Variables|/Game/Blueprints/Game/BP_FirstPersonCharacter.BP_FirstPersonCharacter_C|GetUI%20Controls%20Reference _asbp_first_person_character)))))

(fn ConstructionScript)

(fn GetGlobalControlsType
  (return (Variables|/Game/Blueprints/Game/BP_GameInstance.BP_GameInstance_C|GetControls%20Type (.AsBP%20Game%20Instance (Utilities|Casting|CastToBP_GameInstance (Game|GetGameInstance))))))