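; Mobile player controller that sets up touch controls from the game instance's ControlsType: virtual joysticks or a maps-style "360° Media" mode.
; In 360° mode, dragging rotates the camera and feeds a weighted velocity that a looping timer decays as drift after release.
; Double-tap moves the character to the navmesh-projected touch point, or stops it if moving.
; Spreading two fingers zooms via negative spring arm length, reset on release, in either mode.
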(event Custom|Camera%20Drift
  ;[1 0.08333 0.08333 0.865] Drifting Camera after releasing touch scrolling (Delegate-only Event. Tick can't add input or rotate Camera)
  (if (> (Math|Vector2D|Vector2DLength (Variables|Default|GetWeighted%20Velocity)) 0.1)
    (bind _output_get (Variables|Default|SetWeighted%20Velocity (* (Variables|Default|GetWeighted%20Velocity) (- 1.0 (Variables|Default|GetCamera%20Friction))))) ; Update Velocity at Tick pace
    (Class|PlayerController|AddYawInput (.x _output_get)) ; X-Axis
    (Class|PlayerController|AddPitchInput (.y _output_get)) ; Y-Axis
    (else
      (Utilities|Time|ClearandInvalidateTimerbyHandle (stale Input|EnhancedActionEvents|EnhancedInputActionIA_LookTouch _returnvalue_2)) ; Drift stop
    )))

(event Input|EnhancedActionEvents|EnhancedInputActionIA_PinchZoom
  (params (ActionValue :type Float%20%28double-precision%29) (ElapsedSeconds :type Float%20%28double-precision%29) (TriggeredSeconds :type Float%20%28double-precision%29) (InputAction :type Input%20Action%20Object%20Reference :default "/Game/Input/Actions/IA_PinchZoom.IA_PinchZoom"))
  (:Triggered
    ;[0.03955 0.6584 0] Apply Zoom
    (if (< (* (- (CallFunction|ComputePinchDistance) (Variables|Default|GetInitial%20Pinch)) -1.0) 0.0)
      (CallFunction|Zoom (* (- (CallFunction|ComputePinchDistance) (Variables|Default|GetInitial%20Pinch)) -1.0))))
  (:Started
    (Variables|Default|SetInitial%20Pinch (CallFunction|ComputePinchDistance)))
  (:Completed
    (CallFunction|Zoom 0.0) ; Reset zoom
  ))

(event Input|EnhancedActionEvents|EnhancedInputActionIA_LookTouch
  (params (ActionValue :type Boolean) (ElapsedSeconds :type Float%20%28double-precision%29) (TriggeredSeconds :type Float%20%28double-precision%29) (InputAction :type Input%20Action%20Object%20Reference :default "/Game/Input/Actions/IA_LookTouch.IA_LookTouch"))
  (bind (_locationx _locationy _biscurrentlypressed) (Class|PlayerController|GetInputTouchState "Touch1"))
  (bind _returnvalue (Math|Vector2D|MakeVector2D _locationx _locationy))
  (:Triggered
    (switch Utilities|FlowControl|Switch|SwitchonEnum_ControlTypes (CallFunction|GetGlobalControlsType)
      (:NewEnumerator0
        ;[1 1 1] Scroll to look
        (if (and _biscurrentlypressed (not (.bIsCurrentlyPressed (Class|PlayerController|GetInputTouchState "Touch2")))) ; Only do if touch pressed
          (bind _output_get (Variables|Default|SetDrag%20Velocity (* (- (Variables|Default|GetTouch%20Position) _returnvalue) (Variables|Default|GetScreen%20to%20Camera%20Coords%20Factor)))) ; Compute Velocity
          (Class|PlayerController|AddYawInput (.x _output_get)) ; X-Axis
          (Class|PlayerController|AddPitchInput (.y _output_get)) ; Y-Axis
          (Variables|Default|SetTouch%20Position _returnvalue) ; Update position each frame
          (Variables|Default|SetWeighted%20Velocity (+ (* (Variables|Default|GetWeighted%20Velocity) (Variables|Default|GetDamping%20Coefficient)) (* (Variables|Default|GetDrag%20Velocity) (- 1.0 (Variables|Default|GetDamping%20Coefficient))))) ; Compute temporal average
        ))))
  (:Completed
    (switch Utilities|FlowControl|Switch|SwitchonEnum_ControlTypes (CallFunction|GetGlobalControlsType)
      (:NewEnumerator0
        ;[1 0.08333 0.08333 0.865] Drifting Camera after releasing touch scrolling (Delegate-only Event. Tick can't add input or rotate Camera)
        (bind _returnvalue_2 (Utilities|Time|SetTimerbyEvent (delegate Custom|Camera%20Drift) (Utilities|Time|GetWorldDeltaSeconds) true)) ; Analog behavour as with Tick
      ))))

(event EventBeginPlay
  (switch Utilities|FlowControl|Switch|SwitchonEnum_ControlTypes (CallFunction|GetGlobalControlsType)
    (:NewEnumerator0
      (Class|PlayerController|ActivateTouchInterface) ; NULL: Disable Virtual Joysticks
    )
    (:NewEnumerator1
      (Class|PlayerController|ActivateTouchInterface "/Engine/MobileResources/HUD/DefaultVirtualJoysticks.DefaultVirtualJoysticks"))))

(event Input|TouchEvents|Touch1
  (params (Key :type Key%20Structure))
  (bind (_locationx _locationy) (Class|PlayerController|GetInputTouchState "Touch1"))
  (bind _hitresult (Class|PlayerController|GetHitResultUnderFingerbyChannel "Touch1" "TraceTypeQuery1" false))
  (bind (_projectedlocation _returnvalue) (AI|Navigation|ProjectPointtoNavigation (.location _hitresult) 0 0 "0, 0, 0"))
  (:Pressed
    (switch Utilities|FlowControl|Switch|SwitchonEnum_ControlTypes (CallFunction|GetGlobalControlsType)
      (:NewEnumerator0
        (Utilities|FlowControl|Sequence
          (:then_0
            ;[1 1 1] Acquire initial touch position
            (Variables|Default|SetTouch%20Position (Math|Vector2D|MakeVector2D _locationx _locationy)))
          (:then_1
            ;[1 0.5906 0.01681] Set next movement location based on touched point
            (if _returnvalue
              (Variables|Default|SetMovement%20Location _projectedlocation)
              (else
                (Variables|Default|SetMovement%20Location (Transformation|GetActorLocation (Game|GetPlayerCharacter 0))) ; Don't move if double tap in wrong spot.
              )))
          (:then_2
            ;[0.0137 0.7682 0.4287] Resets double-tap if too slow
            (bind _output_get (Variables|DoubleTap|SetTouch%20Pressed%20Time (Utilities|Time|GetGameTimeinSeconds)))
            (if (> (- _output_get (Variables|DoubleTap|GetTouch%20Released%20Time)) (Variables|DoubleTap|GetDouble%20Tap%20Interval))
              (Variables|DoubleTap|SetDouble%20Tap%20Amount 0) ; Too much time passed: resetting double-tap
            ))))))
  (:Released
    (switch Utilities|FlowControl|Switch|SwitchonEnum_ControlTypes (CallFunction|GetGlobalControlsType)
      (:NewEnumerator0
        (Utilities|FlowControl|Sequence
          (:then_0
            ;[0.0137 0.7682 0.4287] Evaluate if double-tap is happening on touch released
            (bind _output_get_2 (Variables|DoubleTap|SetTouch%20Released%20Time (Utilities|Time|GetGameTimeinSeconds)))
            (if (< (- _output_get_2 (Variables|DoubleTap|GetTouch%20Pressed%20Time)) (Variables|DoubleTap|GetDouble%20Tap%20Interval))
              (Math|Integer|IncrementInt (Variables|DoubleTap|GetDouble%20Tap%20Amount))))
          (:then_1
            ;[0 0.3968 0.8963] Double-tap logic
            (if (== (Variables|DoubleTap|GetDouble%20Tap%20Amount) 2) ; If double-tap happened
              (Variables|DoubleTap|SetDouble%20Tap%20Amount 0) ; Reset double-tap
              (if (CallFunction|IsCharacterMoving)
                (AI|Navigation|StopMovement) ; Character IS moving -> Stop
                (else
                  (AI|Navigation|SimpleMovetoLocation self (Variables|Default|GetMovement%20Location)) ; Character NOT moving -> Move
                )))))))))

(fn ConstructionScript)

(fn InputSetFirstTouchPosition
  (bind (_locationx _locationy) (Class|PlayerController|GetInputTouchState "Touch1"))
  (Variables|Default|SetTouch%20Position (Math|Vector2D|MakeVector2D _locationx _locationy)))

(fn IsCharacterMoving
  (return (> (Math|Vector|VectorLength (Transformation|GetVelocity (Game|GetPlayerCharacter 0))) 0.0)))

(fn GetGlobalControlsType
  (return (.Controls%20Type (Variables|/Game/Blueprints/Game/BP_GameInstance.BP_GameInstance_C|GetControls%20Type (.AsBP%20Game%20Instance (Utilities|Casting|CastToBP_GameInstance (Game|GetGameInstance)))))))

(fn Zoom
  (params (Spring%20Arm%20Length :type Float%20%28single-precision%29))
  (Variables|/Script/Engine.SpringArmComponent|SetTargetArmLength (Variables|/Script/AndroidTestProject.AndroidTestProjectCharacter|GetSpringArm (.AsBP%20First%20Person%20Character (Utilities|Casting|CastToBP_FirstPersonCharacter (Game|GetPlayerCharacter 0)))) Spring%20Arm%20Length))

(fn ComputePinchDistance
  (bind (_locationx _locationy) (Class|PlayerController|GetInputTouchState "Touch2"))
  (bind (_locationx_2 _locationy_2) (Class|PlayerController|GetInputTouchState "Touch1"))
  (return (Math|Vector2D|Vector2DLength (- (Math|Vector2D|MakeVector2D _locationx_2 _locationy_2) (Math|Vector2D|MakeVector2D _locationx _locationy)))))

(fn GetSpringArmLength
  (return (Variables|/Script/Engine.SpringArmComponent|GetTargetArmLength (Variables|/Script/AndroidTestProject.AndroidTestProjectCharacter|GetSpringArm (.AsBP%20First%20Person%20Character (Utilities|Casting|CastToBP_FirstPersonCharacter (Game|GetPlayerCharacter 0)))))))